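; Chess-style board piece whose construction script builds a mesh and dynamic material from Figure and Side, with side-specific textures for Queen and Rook.
; Hovering tints it yellow; clicking hides all BoardTiles, then reveals and highlights those passing that figure's rule, without moving the piece.
; Rules are simplified: Bishop matches rows and columns, Rook an index offset of nine, while Queen and Knight always return false.
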(event OnClicked(Collision)
  (params (TouchedComponent :type Primitive%20Component%20Object%20Reference) (ButtonPressed :type Key%20Structure :default "None"))
  (bind _outactors (Actor|GetAllActorsOfClass "/Game/Blueprints/BoardTile.BoardTile_C"))
  (for _array_element _outactors
    (Variables|Default|SetTile _array_element)
    (Variables|/Game/Blueprints/BoardTile.BoardTile_C|SetVisible _array_element false)
    (switch Utilities|FlowControl|Switch|SwitchonFigures (Variables|Default|GetFigure)
      (:NewEnumerator0
        (bind _canbe (CallFunction|CanbeUsedbyPawn))
        (if _canbe
          (Rendering|Material|SetVectorParameterValue (Variables|/Game/Blueprints/BoardTile.BoardTile_C|GetTileMaterial _array_element) "Emission" "(R=1.000000,G=0.965491,B=0.000000,A=1.000000)" :!class /Script/Engine.MaterialInstanceDynamic :!label _label)
          (Variables|/Game/Blueprints/BoardTile.BoardTile_C|SetVisible _array_element true)))
      (:NewEnumerator1
        (bind _canbe_2 (CallFunction|CanbeUsedbyBishop))
        (if _canbe_2
          (goto _label)))
      (:NewEnumerator6
        (bind _canbe_3 (CallFunction|CanbeUsedbyKing))
        (if _canbe_3
          (goto _label)))
      (:NewEnumerator2
        (bind _canbe_4 (CallFunction|CanbeUsedbyQueen))
        (if _canbe_4
          (goto _label)))
      (:NewEnumerator3
        (bind _canbe_5 (CallFunction|CanbeUsedbyKnight))
        (if _canbe_5
          (goto _label)))
      (:NewEnumerator4
        (bind _canbe_6 (CallFunction|CanbeUsedbyRook))
        (if _canbe_6
          (goto _label))))))

(event OnBeginCursorOver(Collision)
  (params (TouchedComponent :type Primitive%20Component%20Object%20Reference))
  (Rendering|Material|SetVectorParameterValue (Variables|Default|GetFigure%20Material) "Tint" "(R=1.000000,G=0.834791,B=0.000000,A=1.000000)" :!class /Script/Engine.MaterialInstanceDynamic))

(event OnEndCursorOver(Collision)
  (params (TouchedComponent :type Primitive%20Component%20Object%20Reference))
  (Rendering|Material|SetVectorParameterValue (Variables|Default|GetFigure%20Material) "Tint" (Variables|Default|GetInitialTint) :!class /Script/Engine.MaterialInstanceDynamic))

(event EventBeginPlay
  (bind _returnvalue (Rendering|Material|GetVectorParameterValue (Variables|Default|GetFigure%20Material) "Tint" :!class /Script/Engine.MaterialInstanceDynamic))
  (Variables|Default|SetInitialTint _returnvalue))

(fn ConstructionScript
  (bind _side (Variables|Default|GetSide))
  (switch Utilities|FlowControl|Switch|SwitchonFigures (Variables|Default|GetFigure)
    (:NewEnumerator0
      (bind _returnvalue (AddComponent|AddStaticMeshComponent false))
      (bind _returnvalue_2 (Rendering|Material|CreateDynamicMaterialInstance _returnvalue 0 "/Game/Meshes/Lewis/M_Figure.M_Figure" "None" :!class /Script/Engine.PrimitiveComponent))
      (bind _output_get (Variables|Default|SetFigure%20Material _returnvalue_2))
      (Rendering|Material|SetTextureParameterValue _output_get "Texture" "/Game/Meshes/Lewis/pawn_1.pawn_1"))
    (:NewEnumerator1
      (bind _returnvalue_3 (AddComponent|AddStaticMeshComponent false))
      (bind _returnvalue_4 (Rendering|Material|CreateDynamicMaterialInstance _returnvalue_3 0 "/Game/Meshes/Lewis/M_Figure.M_Figure" "None" :!class /Script/Engine.PrimitiveComponent))
      (bind _output_get_2 (Variables|Default|SetFigure%20Material _returnvalue_4))
      (Rendering|Material|SetTextureParameterValue _output_get_2 "Texture" "/Game/Meshes/Lewis/bishop_1.bishop_1"))
    (:NewEnumerator6
      (bind _returnvalue_5 (AddComponent|AddStaticMeshComponent false))
      (bind _returnvalue_6 (Rendering|Material|CreateDynamicMaterialInstance _returnvalue_5 0 "/Game/Meshes/Lewis/M_Figure.M_Figure" "None" :!class /Script/Engine.PrimitiveComponent))
      (bind _output_get_3 (Variables|Default|SetFigure%20Material _returnvalue_6))
      (Rendering|Material|SetTextureParameterValue _output_get_3 "Texture" "/Game/Meshes/Lewis/king_1.king_1"))
    (:NewEnumerator2
      (if _side
        (bind _returnvalue_7 (AddComponent|AddStaticMeshComponent false))
        (bind _returnvalue_8 (Rendering|Material|CreateDynamicMaterialInstance _returnvalue_7 0 "/Game/Meshes/Lewis/M_Figure.M_Figure" "None" :!class /Script/Engine.PrimitiveComponent))
        (bind _output_get_4 (Variables|Default|SetFigure%20Material _returnvalue_8))
        (Rendering|Material|SetTextureParameterValue _output_get_4 "Texture" "/Game/Meshes/Lewis/queen_2.queen_2")
        (else
          (bind _returnvalue_9 (AddComponent|AddStaticMeshComponent false))
          (bind _returnvalue_10 (Rendering|Material|CreateDynamicMaterialInstance _returnvalue_9 0 "/Game/Meshes/Lewis/M_Figure.M_Figure" "None" :!class /Script/Engine.PrimitiveComponent))
          (bind _output_get_5 (Variables|Default|SetFigure%20Material _returnvalue_10))
          (Rendering|Material|SetTextureParameterValue _output_get_5 "Texture" "/Game/Meshes/Lewis/queen_1.queen_1"))))
    (:NewEnumerator3
      (bind _returnvalue_11 (AddComponent|AddStaticMeshComponent false))
      (bind _returnvalue_12 (Rendering|Material|CreateDynamicMaterialInstance _returnvalue_11 0 "/Game/Meshes/Lewis/M_Figure.M_Figure" "None" :!class /Script/Engine.PrimitiveComponent))
      (bind _output_get_6 (Variables|Default|SetFigure%20Material _returnvalue_12))
      (Rendering|Material|SetTextureParameterValue _output_get_6 "Texture" "/Game/Meshes/Lewis/knight_1.knight_1"))
    (:NewEnumerator4
      (if _side
        (bind _returnvalue_13 (AddComponent|AddStaticMeshComponent false))
        (bind _returnvalue_14 (Rendering|Material|CreateDynamicMaterialInstance _returnvalue_13 0 "/Game/Meshes/Lewis/M_Figure.M_Figure" "None" :!class /Script/Engine.PrimitiveComponent))
        (bind _output_get_7 (Variables|Default|SetFigure%20Material _returnvalue_14))
        (Rendering|Material|SetTextureParameterValue _output_get_7 "Texture" "/Game/Meshes/Lewis/berserker_1.berserker_1")
        (else
          (bind _returnvalue_15 (AddComponent|AddStaticMeshComponent false))
          (bind _returnvalue_16 (Rendering|Material|CreateDynamicMaterialInstance _returnvalue_15 0 "/Game/Meshes/Lewis/M_Figure.M_Figure" "None" :!class /Script/Engine.PrimitiveComponent))
          (bind _output_get_8 (Variables|Default|SetFigure%20Material _returnvalue_16))
          (Rendering|Material|SetTextureParameterValue _output_get_8 "Texture" "/Game/Meshes/Lewis/berserker_2.berserker_2")))))
  (if (not (Variables|Default|GetSide))
    (Rendering|Material|SetVectorParameterValue (Variables|Default|GetFigure%20Material) "Tint" "(R=1.000000,G=1.000000,B=1.000000,A=1.000000)" :!class /Script/Engine.MaterialInstanceDynamic)))

(fn CanbeUsedbyPawn
  (bind _tile (Variables|Default|GetTile))
  (bind _index (Variables|Default|GetIndex))
  (bind _index_2 (Variables|/Game/Blueprints/BoardTile.BoardTile_C|GetIndex _tile))
  (bind _returnvalue (- _index_2 _index))
  (if (Variables|Default|GetSide)
    (return (== _returnvalue 8))
    (else
      (return (== _returnvalue -8)))))

(fn CanbeUsedbyKing
  (bind _tile (Variables|Default|GetTile))
  ;[1 1 1] Pawn tiles
  (return (and (Utilities|InRangeOfOne (Variables|Default|GetX) (Variables|/Game/Blueprints/BoardTile.BoardTile_C|GetX _tile)) (Utilities|InRangeOfOne (Variables|Default|GetY) (Variables|/Game/Blueprints/BoardTile.BoardTile_C|GetY _tile)))))

(fn CanbeUsedbyBishop
  (bind _tile (Variables|Default|GetTile))
  (return (or (== (Variables|/Game/Blueprints/BoardTile.BoardTile_C|GetX _tile) (Variables|Default|GetX)) (== (Variables|/Game/Blueprints/BoardTile.BoardTile_C|GetY _tile) (Variables|Default|GetY)))))

(fn CanbeUsedbyQueen
  (return false))

(fn CanbeUsedbyRook
  (return (or (== (Math|Integer|Absolute(Integer) (- (Variables|/Game/Blueprints/BoardTile.BoardTile_C|GetIndex (Variables|Default|GetTile)) (Variables|Default|GetIndex))) 9) false)))

(fn CanbeUsedbyKnight
  (return false))