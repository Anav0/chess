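; BoardTile is a single board tile with a mesh and a text label showing its X and Y coordinates.
; The construction script creates a dynamic M_Tile material instance for the mesh, joins X and Y without a separator for the label, and sets Visible to true.
; Tick applies the Visible flag to the tile mesh every frame, without propagating it to child components.
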(event EventTick
  (params (DeltaSeconds :type Float%20%28single-precision%29))
  (Rendering|SetVisibility (Variables|Default|GetTileMesh) (Variables|Default|GetVisible) false))

(fn ConstructionScript
  (bind _returnvalue (Rendering|Material|CreateDynamicMaterialInstance "/Game/Meshes/M_Tile.M_Tile" "None" "None" :!class /Script/Engine.KismetMaterialLibrary))
  (bind _output_get (Variables|Default|SetTileMaterial _returnvalue))
  (Rendering|Material|SetMaterial (Variables|Default|GetTileMesh) 0 _output_get)
  (Rendering|Components|TextRender|SetText (Variables|Default|GetTextRender) (Utilities|Text|ToText(String) (Utilities|String|Append (Utilities|String|ToString(Integer) (Variables|Default|GetX)) (Utilities|String|ToString(Integer) (Variables|Default|GetY)))))
  (Variables|Default|SetVisible true))