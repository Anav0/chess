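; Chess board actor that builds the 8x8 grid of tiles and places the starting pieces at BeginPlay.
; A nested loop spawns each tile at a fixed spacing from the board's transform, passing it grid coordinates and a running index.
; DeterminFigureType picks the piece from row and column, using position lists for rooks, knights and bishops.
; Each piece spawns on its tile, with side and yaw derived from the row.
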(event EventBeginPlay
  (bind _board (Variables|Default|Getboard))
  (bind _returnvalue (Transformation|GetWorldTransform _board))
  (switch Utilities|FlowControl|Switch|SwitchonBoardType "NewEnumerator0"
    (:NewEnumerator0
      (Variables|Default|SetTileTransform (Math|Transform|MakeTransform (Math|Vector|MakeVector (+ (.x (.location _returnvalue)) 44.0) (+ (.y (.location _returnvalue)) 44.0) (+ (.z (.location _returnvalue)) 3.0)) "0.000000,90.000000,0.000000" "0.200000,0.200000,1.000000"))
      (Variables|Default|SetGap -9.85)
      (bind _index (Utilities|FlowControl|ForLoopwithBreak 1 8)
        (:LoopBody
          (Variables|Default|SetX _index)
          (bind _index_2 (Utilities|FlowControl|ForLoopwithBreak 1 8)
            (:LoopBody
              (Variables|Default|SetY _index_2)
              (Variables|Default|SetTileIndex (+ (Variables|Default|GetTileIndex) 1))
              (bind _returnvalue_2 (Game|SpawnActorfromClass "/Game/Blueprints/BoardTile.BoardTile_C" (Math|Transform|MakeTransform (Math|Vector|MakeVector (+ (.x (.location (Variables|Default|GetTileTransform))) (* (Variables|Default|GetX) (Variables|Default|GetGap))) (+ (.y (.location (Variables|Default|GetTileTransform))) (* (Variables|Default|GetGap) (Variables|Default|GetY))) (.z (.location (Variables|Default|GetTileTransform)))) (.rotation (Variables|Default|GetTileTransform)) (.scale (Variables|Default|GetTileTransform))) "Undefined" 0 (Variables|Default|GetX) (Variables|Default|GetY) (Variables|Default|GetTileIndex) 0))
              (bind (_type _havefigure) (CallFunction|DeterminFigureType))
              (if _havefigure
                (if (>= (Variables|Default|GetX) 3)
                  (Variables|Default|SetPiceRotation 9e+01)
                  (else
                    (Variables|Default|SetPiceRotation -9e+01)))
                (Game|SpawnActorfromClass "/Game/Blueprints/Pice.Pice_C" (Math|Transform|MakeTransform (Transformation|GetWorldLocation (Variables|/Script/Engine.Actor|GetRootComponent _returnvalue_2)) (Math|Rotator|MakeRotator 0.0 0.0 (Variables|Default|GetPiceRotation)) "1,1,1") "Undefined" 0 _type (>= (Variables|Default|GetX) 3) (Variables|Default|GetX) (Variables|Default|GetY) (Variables|Default|GetTileIndex) 0)))))))))

(event Collision|EventActorBeginOverlap
  (params (OtherActor :type Actor%20Object%20Reference)))

(event EventTick
  (params (DeltaSeconds :type Float%20%28single-precision%29)))

(fn ConstructionScript)

(fn DeterminFigureType
  (bind _x (Variables|Default|GetX))
  (bind _x_2 (Variables|Default|GetX))
  (bind _y (Variables|Default|GetY))
  (if (or (== _x_2 7) (== _x_2 2))
    (return "NewEnumerator0" true)
    (elif (or (== _x 1) (== _x 8))
      (if (== (Variables|Default|GetY) 4)
        (bind _output_get (Variables|Default|SetPice "NewEnumerator6"))
        (return _output_get true)
        (elif (== (Variables|Default|GetY) 5)
          (bind _output_get_2 (Variables|Default|SetPice "NewEnumerator2"))
          (return _output_get_2 true)
          (elif (Utilities|Set|Contains (Variables|Default|GetRookPos) _y)
            (bind _output_get_3 (Variables|Default|SetPice "NewEnumerator4"))
            (return _output_get_3 true)
            (elif (Utilities|Set|Contains (Variables|Default|GetKnightPos) _y)
              (bind _output_get_4 (Variables|Default|SetPice "NewEnumerator3"))
              (return _output_get_4 true)
              (elif (Utilities|Set|Contains (Variables|Default|GetBishopPos) _y)
                (bind _output_get_5 (Variables|Default|SetPice "NewEnumerator1"))
                (return _output_get_5 true)
                (else
                  (return "NewEnumerator0" false)))))))
      (else
        (return "NewEnumerator0" false)))))